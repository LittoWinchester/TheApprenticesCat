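; BP_Cat is an interactable actor that shows a UI_Cat widget and mouse cursor when the player character interacts within range.
; BeginPlay creates the cat widget and a Press E prompt, which are added on actor overlap and removed when the Box overlap ends.
; While overlapping, Tick polls BP_Character's InteractioOn flag to swap between prompt and cat UI; entering or leaving resets that flag.
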(event `x`)

(event `x2`
  (`Widget.SetVisibility` (`self.Cat UI`) "Visible"))

(event `HideUI`
  ;[1 1 1] Show and Hide
  (`Widget.SetVisibility` (`self.Cat UI`) "Hidden"))

(event `ShowUI`
  ;[1 1 1] Show and Hide
  (`Widget.SetVisibility` (`self.Cat UI`) "Visible"))

(event `self.ReceiveBeginPlay`
  (bind _returnvalue (`|CreateWidget` "/Game/UI/UI_Cat.UI_Cat_C" (`GameplayStatics.GetPlayerController` 0)))
  (set `self.Cat UI` _returnvalue)
  (bind _returnvalue_2 (`|CreateWidget` "/Game/UI/UI_PressE.UI_PressE_C"))
  (set `self.Press_E` _returnvalue_2))

(event `self.ReceiveTick`
  (params (DeltaSeconds :type "Float (single-precision)"))
  (bind _returnvalue (`GameplayStatics.GetPlayerController` 0))
  (bind _press_e (`self.Press_E`))
  ;[1 1 1] Tick / show when collapse
  (if (`self.Overlaping`)
    (bind _asbp_character (cast `/Game/Blueprints/BP_Character` (`GameplayStatics.GetPlayerCharacter` 0)))
    (if (`/Game/Blueprints/BP_Character.interactio_on` _asbp_character)
      (set `PlayerController.bShowMouseCursor` true _returnvalue)
      (`self.ShowUI`)
      (`Widget.SetVisibility` _press_e "Hidden")
      (else
        (set `PlayerController.bShowMouseCursor` false _returnvalue)
        (`self.HideUI`)
        (`Widget.SetVisibility` _press_e "Visible")))))

(event `self.ReceiveActorBeginOverlap`
  (params (OtherActor :type "Actor Object Reference"))
  (bind _cat_ui (`self.Cat UI`))
  ;[1 1 1] Begin and Overlap
  (if (== OtherActor (`GameplayStatics.GetPlayerCharacter` 0))
    (`UserWidget.AddToViewport` (`self.Press_E`) 0)
    (set `self.Overlaping` true)
    (bind _asbp_character (cast `/Game/Blueprints/BP_Character` (`GameplayStatics.GetPlayerCharacter` 0)))
    (set `/Game/Blueprints/BP_Character.interactio_on` false _asbp_character)
    (`UserWidget.AddToPlayerScreen` _cat_ui 0)
    (`Widget.SetVisibility` _cat_ui "Hidden")))

(event `self.Box.OnComponentEndOverlap`
  (params (OverlappedComponent :type "PrimitiveComponent Object Reference") (OtherActor :type "Actor Object Reference") (OtherComp :type "PrimitiveComponent Object Reference") (OtherBodyIndex :type Integer))
  ;[1 1 1] Begin and Overlap
  (if (== (`GameplayStatics.GetPlayerCharacter` 0) OtherActor)
    (`Widget.RemoveFromParent` (`self.Press_E`))
    (`Widget.RemoveFromParent` (`self.Cat UI`))
    (set `self.Overlaping` false)
    (bind _asbp_character (cast `/Game/Blueprints/BP_Character` (`GameplayStatics.GetPlayerCharacter` 0)))
    (set `/Game/Blueprints/BP_Character.interactio_on` false _asbp_character)))

(fn `UserConstructionScript`)